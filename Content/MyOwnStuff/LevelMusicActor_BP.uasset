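; Level music actor that plays a sound and drives audio-reactive cubes in time with it.
; On BeginPlay it starts the audio component at a 40-second offset and listens to playback percent, converting it to elapsed time.
; Each update samples a Constant-Q spectrum at that time and sets the Z scale of the matching cube from each band.
; The construction script gathers all AudioReactiveCubes in the level into the array.
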(event `self.ReceiveBeginPlay`
  (`AudioComponent.SetSound` (`self.Audio`) (`self.Sound`))
  (set `self.Duration` (`SoundBase.Duration` (`self.Sound`)))
  (add `AudioComponent.OnAudioPlaybackPercent` (`self.Audio`) (delegate `PlaybackChange`))
  (`AudioComponent.Play` (`self.Audio`) 40.0))

(event `PlaybackChange`
  (params (PlayingSoundWave :type "SoundWave Object Reference") (PlaybackPercent :type "Float (double-precision)"))
  (set `self.PlayedTime` (* PlaybackPercent (`self.Duration`)))
  (for (_array_element _array_index) (`ConstantQNRT.GetNormalizedChannelConstantQAtTime` (`self.Constant_Ref`) (`self.PlayedTime`) 0)
    (bind _output (`|GetArrayItem` (`self.AudioCubes`) _array_index))
    (`/Engine/EditorBlueprintResources/StandardMacros.IsValid` _output
      (:`Is Valid`
        (bind (_returnvalue_x _returnvalue_y _returnvalue_z) (`KismetMathLibrary.BreakVector` (* (`KismetMathLibrary.Conv_DoubleToVector` _array_element) 2.0)))
        (`SceneComponent.SetWorldScale3D` (`/Game/MyOwnStuff/AudioReactiveStuff/AudioReactiveCubes.Cube` _output) (`KismetMathLibrary.MakeVector` 0.5 0.5 _returnvalue_z))
        (set `self.SoundRead` _array_element)))))

(fn `UserConstructionScript`
  (bind _outactors (`GameplayStatics.GetAllActorsOfClass` "/Game/MyOwnStuff/AudioReactiveStuff/AudioReactiveCubes.AudioReactiveCubes_C"))
  (set `self.AudioCubes` _outactors))