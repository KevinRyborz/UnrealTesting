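; AudioLight_BP is an audio-reactive spotlight that pulses with the level music.
; On BeginPlay it finds the LevelMusicActor_BP in the level, keeps a reference to it and applies a starting intensity.
; Every Tick it scales the spotlight's intensity and outer cone angle by that actor's SoundRead value, with the inner cone held at a third of the outer.
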(event `self.ReceiveBeginPlay`
  (bind _returnvalue (`GameplayStatics.GetActorOfClass` "/Game/MyOwnStuff/LevelMusicActor_BP.LevelMusicActor_BP_C"))
  (set `self.LevelMusicReference` _returnvalue)
  (`LightComponent.SetIntensity` (`self.SpotLight`) (`self.StartIntensity`)))

(event `self.ReceiveTick`
  (params (DeltaSeconds :type "Float (single-precision)"))
  (bind _spotlight (`self.SpotLight`))
  (bind _soundread (`/Game/MyOwnStuff/LevelMusicActor_BP.SoundRead` (`self.LevelMusicReference`)))
  (bind _returnvalue (* 50 _soundread))
  (`LightComponent.SetIntensity` (`self.SpotLight`) (* 100000 _soundread))
  (`SpotLightComponent.SetOuterConeAngle` _spotlight _returnvalue)
  (`SpotLightComponent.SetInnerConeAngle` _spotlight (/ _returnvalue 3.0)))

(fn `UserConstructionScript`)