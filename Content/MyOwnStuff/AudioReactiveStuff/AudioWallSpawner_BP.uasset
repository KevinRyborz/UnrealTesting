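; AudioWallSpawner_BP is a spawner actor that emits AudioWall actors whose height reacts to the level's audio.
; It caches LevelMusicActor_BP on BeginPlay, then scales each wall's Z by that actor's SoundRead times a multiplier.
; While SpawnWall is set, a Delay on Tick paces spawning at the root's location.
; Each new wall receives its position deltas and destroy time from the spawner's variables.
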(event `self.ReceiveBeginPlay`
  (bind _returnvalue (`GameplayStatics.GetActorOfClass` "/Game/MyOwnStuff/LevelMusicActor_BP.LevelMusicActor_BP_C"))
  (set `self.LevelMusicReference` _returnvalue))

(event `self.ReceiveTick`
  (params (DeltaSeconds :type "Float (single-precision)"))
  (if (`self.SpawnWall?`)
    (`KismetSystemLibrary.Delay` (`self.TimeUntilNewElement`))
    (bind _returnvalue (`|SpawnActorFromClass` "/Game/MyOwnStuff/AudioReactiveStuff/AudioWall.AudioWall_C" (`KismetMathLibrary.MakeTransform` (`SceneComponent.K2_GetComponentLocation` (`self.DefaultSceneRoot`)) (struct) (`KismetMathLibrary.MakeVector` (`self.X Transform`) (`self.Y Transform`) (* (`/Game/MyOwnStuff/LevelMusicActor_BP.SoundRead` (`self.LevelMusicReference`)) (`self.Z Transform Multiplier`)))) "Undefined" "OverrideRootScale" null null))
    (set `/Game/MyOwnStuff/AudioReactiveStuff/AudioWall.DeltaLocX` (`self.Wall Pos X`) _returnvalue)
    (set `/Game/MyOwnStuff/AudioReactiveStuff/AudioWall.DeltaLocY` (`self.Wall Pos Y`) _returnvalue)
    (set `/Game/MyOwnStuff/AudioReactiveStuff/AudioWall.DeltaLocZ` (`self.Wall Pos Z`) _returnvalue)
    (set `/Game/MyOwnStuff/AudioReactiveStuff/AudioWall.TimeUntilDestroy` (`self.TimeUntilDestroyRef`) _returnvalue)))

(fn `UserConstructionScript`)