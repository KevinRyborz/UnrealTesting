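; Trigger-zone actor that lets the player toggle music and two attached Niagara particle effects, apparently audio-reactive by their names.
; First-person character overlap shows a text prompt and starts an endless 0.2-second delay loop polling InTrigger; leaving hides the prompt.
; The Interact input flip-flops a flag.
; While inside, InTrigger uses it to play audio from an offset and spawn both systems once, or stop and destroy them.
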(event `self.ReceiveBeginPlay`
  (`SceneComponent.SetVisibility` (`self.TextPrompt`) false false)
  (`self.EnableInput` (`GameplayStatics.GetPlayerController` 0))
  (set `self.Spawned System Lava` null)
  (set `self.Spawned System Green` null))

(event `InputAction|Interact`
  (params (Key :type "Key Structure"))
  (:`Pressed`
    (`/Engine/EditorBlueprintResources/StandardMacros.FlipFlop`
      (:`A`
        (set `self.Interact` true))
      (:`B`
        (set `self.Interact` false)))))

(event `self.ReceiveActorBeginOverlap`
  (params (OtherActor :type "Actor Object Reference"))
  (cast `/Game/FirstPersonBP/Blueprints/FirstPersonCharacter` OtherActor)
  (set `self.isInTrigger` true)
  (`self.InTrigger` :!label _label)
  (`KismetSystemLibrary.Delay` 0.2)
  (goto _label))

(event `self.ReceiveActorEndOverlap`
  (params (OtherActor :type "Actor Object Reference"))
  (cast `/Game/FirstPersonBP/Blueprints/FirstPersonCharacter` OtherActor)
  (set `self.isInTrigger` false)
  (`self.InTrigger`))

(event `InTrigger`
  (if (`self.isInTrigger`)
    (`SceneComponent.SetVisibility` (`self.TextPrompt`) true false)
    (if (`self.Interact`)
      (`/Engine/EditorBlueprintResources/StandardMacros.DoOnce` false :!label _label_2
        (:`Completed`
          (`AudioComponent.Play` (`self.Audio`) 50.0)
          (bind _returnvalue (`NiagaraFunctionLibrary.SpawnSystemAttached` "/Game/MyOwnStuff/Particles/AudioReactiveParticles/ReactiveOrchestra.ReactiveOrchestra" (`self.ParticleLocation`) "None" (0.0 0.0 0.0) (struct) "KeepRelativeOffset" true))
          (set `self.Spawned System Lava` _returnvalue)
          (bind _returnvalue_2 (`NiagaraFunctionLibrary.SpawnSystemAttached` "/Game/MyOwnStuff/Particles/AudioReactiveParticles/AudioReactiveNiagraTest.AudioReactiveNiagraTest" (`self.ParticleLocation1`) "None" (0.0 0.0 0.0) (struct) "KeepRelativeOffset" true))
          (set `self.Spawned System Green` _returnvalue_2)))
      (else
        (`AudioComponent.Stop` (`self.Audio`))
        (`ActorComponent.K2_DestroyComponent` (`self.Spawned System Lava`))
        (`ActorComponent.K2_DestroyComponent` (`self.Spawned System Green`))
        (goto _label_2 :!via `Reset`)))
    (else
      (`SceneComponent.SetVisibility` (`self.TextPrompt`) false false))))

(fn `UserConstructionScript`)