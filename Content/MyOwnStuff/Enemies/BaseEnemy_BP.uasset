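; BaseEnemy_BP is a base enemy Blueprint that handles taking damage and dying.
; TakeDamage fires LookAtPlayer and HitEvent, subtracts Damage from Health, then either sets IsDead and fires EnemyDie or prints the remaining health for debugging.
; LookAtPlayer, HitEvent and EnemyDie are empty events here, serving as hooks around the shared damage logic.
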(event `self.ReceiveBeginPlay`)

(event `HitEvent`)

(event `EnemyDie`)

(event `LookAtPlayer`)

(event `/Game/MyOwnStuff/Enemies/BPI_Damageable.TakeDamage`
  (params (Damage :type "Float (single-precision)"))
  (`self.LookAtPlayer`)
  (`self.HitEvent`)
  (bind _output_get (set `self.Health` (- (`self.Health`) Damage)))
  (if (<= _output_get 0.0)
    (`KismetSystemLibrary.PrintString` "dead")
    (set `self.IsDead` true)
    (`self.EnemyDie`)
    (else
      (`KismetSystemLibrary.PrintString` (`KismetStringLibrary.Concat_StrStr` "Enemy Health:" (`KismetStringLibrary.Conv_DoubleToString` (`self.Health`)))))))

(fn `UserConstructionScript`)