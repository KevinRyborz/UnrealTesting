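; ShootingCube_BP is an enemy pawn that faces the player on sight and fires cube projectiles.
; PawnSensing detects the FirstPersonCharacter, then the AI controller cached at BeginPlay sets focus on it.
; The same sighting spawns a CubeProjectile at ProjectileSpawnLocation, throttled by a CanShoot flag reset after a short delay.
; EnemyDie destroys the actor, and a leftover look-at rotation node is unconnected.
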(event `self.ReceiveBeginPlay`
  (bind _asai_controller_enemy_bp (cast `/Game/MyOwnStuff/Enemies/AI/AI_Controller_Enemy_BP` (`self.GetController`)))
  (set `self.AIController` _asai_controller_enemy_bp))

(event `self.PawnSensing.OnSeePawn`
  (params (Pawn :type "Pawn Object Reference"))
  (bind _asfirst_person_character (cast `/Game/FirstPersonBP/Blueprints/FirstPersonCharacter` Pawn))
  (`|ExecutionSequence`
    (:`then_0`
      (`/Engine/EditorBlueprintResources/StandardMacros.IsValid` (`self.AIController`)
        (:`Is Valid`
          (`AIController.K2_SetFocus` (`self.AIController`) _asfirst_person_character))
        (:`Is Not Valid`
          (`KismetSystemLibrary.PrintString` "NotValid"))))
    (:`then_1`
      (if (`self.CanShoot`)
        (`|SpawnActorFromClass` "/Game/MyOwnStuff/Enemies/ShootingCube/CubeProjectile.CubeProjectile_C" (`SceneComponent.K2_GetComponentToWorld` (`self.ProjectileSpawnLocation`)) "Undefined" "OverrideRootScale" null null)
        (set `self.CanShoot` false)
        (`KismetSystemLibrary.Delay` 1.0)
        (set `self.CanShoot` true)))))

(event `self.EnemyDie`
  (`self.K2_DestroyActor`))

(fn `UserConstructionScript`)