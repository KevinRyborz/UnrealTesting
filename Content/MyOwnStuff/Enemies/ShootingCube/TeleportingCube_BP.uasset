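; Teleporting cube enemy that shoots projectiles when it sees the first-person character and is destroyed on death.
; On sight it calls SetActorRotation on the character, not itself, and launches a CubeProjectile by impulse, limited by a half-second cooldown.
; BeginPlay caches three move points and picks one at random.
; A timeline meant to lerp between points, re-pick them and spawn a Niagara effect is never triggered.
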(event `self.PawnSensing.OnSeePawn`
  (params (Pawn :type "Pawn Object Reference"))
  (bind _asfirst_person_character (cast `/Game/FirstPersonBP/Blueprints/FirstPersonCharacter` Pawn))
  (`|ExecutionSequence`
    (:`then_0`
      (`self.K2_SetActorRotation` _asfirst_person_character (`KismetMathLibrary.FindLookAtRotation` (`self.K2_GetActorLocation`) (`self.K2_GetActorLocation`)) false))
    (:`then_1`
      (if (`self.CanShoot`)
        (bind _returnvalue (`|SpawnActorFromClass` "/Game/MyOwnStuff/Enemies/ShootingCube/CubeProjectile.CubeProjectile_C" (`SceneComponent.K2_GetComponentToWorld` (`self.ProjectileSpawnLocation`)) "Undefined" "OverrideRootScale" null null))
        (`PrimitiveComponent.AddImpulse` (`/Game/MyOwnStuff/Enemies/ShootingCube/CubeProjectile.Sphere` _returnvalue) (* (`SceneComponent.GetForwardVector` (`self.Cube`)) (`self.ShootForce`)) "None" true)
        (set `self.CanShoot` false)
        (`KismetSystemLibrary.Delay` 0.5)
        (set `self.CanShoot` true)))))

(event `self.EnemyDie`
  (`self.K2_DestroyActor`))

(event `self.ReceiveBeginPlay`
  (set `self.TeleportPoints` (`|MakeArray` (`SceneComponent.K2_GetComponentLocation` (`self.MovePosition1`)) (`SceneComponent.K2_GetComponentLocation` (`self.MovePosition2`)) (`SceneComponent.K2_GetComponentLocation` (`self.MovePosition3`))))
  (`self.GetRandomLocation`))

(fn `GetRandomLocation`
  (set `self.CurrentTeleportPoint` (`KismetMathLibrary.RandomInteger` (`KismetArrayLibrary.Array_Length` (`self.TeleportPoints`)))))

(fn `UserConstructionScript`)