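; A time-freeze zone actor that slows non-player actors inside it to a near standstill.
; On BeginPlay it moves ZoneCollision to the Zone component's location and caches the player's FirstPersonCharacter; the scale-matching node is left disconnected.
; Begin and end overlap events lower and restore each actor's CustomTimeDilation, skipping the player, with debug prints throughout.
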(event `self.ReceiveBeginPlay`
  (`SceneComponent.K2_SetWorldLocation` (`self.Zone Collision`) (`SceneComponent.K2_GetComponentLocation` (`self.Zone`)) false false)
  (bind _asfirst_person_character (cast `/Game/FirstPersonBP/Blueprints/FirstPersonCharacter` (`GameplayStatics.GetPlayerPawn` 0)))
  (bind _output_get (set `self.PlayerRef` _asfirst_person_character))
  (`KismetSystemLibrary.PrintString` (`KismetSystemLibrary.GetDisplayName` _output_get)))

(event `self.ReceiveActorBeginOverlap`
  (params (OtherActor :type "Actor Object Reference"))
  (bind _output_get (set `self.IsPlayer` (== OtherActor (`self.PlayerRef`))))
  (if _output_get
    (`KismetSystemLibrary.PrintString` "isplayer")
    (else
      (set `Actor.CustomTimeDilation` 0.01 OtherActor)
      (`KismetSystemLibrary.PrintString` "Overlap"))))

(event `self.ReceiveActorEndOverlap`
  (params (OtherActor :type "Actor Object Reference"))
  (bind _output_get (set `self.IsPlayer` (== OtherActor (`self.PlayerRef`))))
  (if _output_get
    (`KismetSystemLibrary.PrintString` "isplayer")
    (else
      (set `Actor.CustomTimeDilation` 1.0 OtherActor)
      (`KismetSystemLibrary.PrintString` "Left"))))

(fn `UserConstructionScript`)