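; Enemy pawn that chases the first-person character once its PawnSensing sees it, and leaves blood effects when hurt or killed.
; Any damage spawns a BloodSplatterActor at the damage causer's location, attached to the mesh, then reduces Health.
; At zero health it ragdolls, drops capsule collision, line-traces vertically through the spine to place a surface-aligned BloodPoolActor, and destroys itself after a delay.
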(event `self.ReceiveBeginPlay`)

(event `self.PawnSensing.OnSeePawn`
  (params (Pawn :type "Pawn Object Reference"))
  (bind _asfirst_person_character (cast `/Game/FirstPersonBP/Blueprints/FirstPersonCharacter` Pawn))
  (`|AIMoveTo` self (0.0 0.0 0.0) _asfirst_person_character 30.0
    (:`OnFail`
      (`KismetSystemLibrary.PrintString` "AI_MoveTo failed"))))

(event `self.ReceiveAnyDamage`
  (params (Damage :type "Float (single-precision)") (DamageType :type "DamageType Object Reference") (InstigatedBy :type "Controller Object Reference") (DamageCauser :type "Actor Object Reference"))
  (bind _returnvalue (`|SpawnActorFromClass` "/Game/MyOwnStuff/BloodSplatter/BloodSplatterActor.BloodSplatterActor_C" (`KismetMathLibrary.MakeTransform` (`self.K2_GetActorLocation` DamageCauser)) "Undefined" "OverrideRootScale" null null))
  (`self.K2_AttachToComponent` _returnvalue (`self.Mesh`) "None" "KeepWorld" "KeepWorld" "KeepWorld" true)
  (if (> (`self.Health`) 0.0)
    (bind _output_get (set `self.Health` (- (`self.Health`) Damage)))
    (if (<= _output_get 0.0)
      (`self.Death`))))

(event `Death`
  (bind _mesh (`self.Mesh`))
  (bind _returnvalue (`SceneComponent.GetSocketLocation` _mesh "spine_02"))
  (`PrimitiveComponent.SetSimulatePhysics` _mesh true)
  (`PrimitiveComponent.SetCollisionEnabled` (`self.CapsuleComponent`) "NoCollision")
  (`KismetSystemLibrary.Delay` 0.0)
  (bind _outhit (`KismetSystemLibrary.LineTraceSingle` (+ _returnvalue (0.0 0.0 250.0)) (+ _returnvalue (0.0 0.0 -250.0)) "TraceTypeQuery1" false (`self.ActorsToIgnore`) "None" true (struct :`R` 0.038946 :`B` 1.0 :`A` 1.0)))
  (bind (_bblockinghit _binitialoverlap _time _distance _location _impactpoint _normal _impactnormal) (`GameplayStatics.BreakHitResult` _outhit))
  (`|SpawnActorFromClass` "/Game/MyOwnStuff/BloodSplatter/BloodPoolActor.BloodPoolActor_C" (`KismetMathLibrary.MakeTransform` _location (`KismetMathLibrary.Conv_VectorToRotator` _impactnormal)) "Undefined" "OverrideRootScale" null null)
  (`KismetSystemLibrary.Delay` 15.0)
  (`self.K2_DestroyActor`))

(fn `UserConstructionScript`)